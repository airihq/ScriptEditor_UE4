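; BP_ZText builds multi-line 3D text from one static mesh component per character, spawned in the construction script.
; SetCharacterMesh finds each glyph by searching the data table of the selected font.
; SpawnText spaces glyphs by bounding-box width and kerning, offsets lines by line height, then shifts each line for left, center or right alignment.
; UpdateText and UpdateFont destroy the tracked meshes and respawn the text.
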(fn ConstructionScript
  (Utilities|Array|Clear (Variables|Default|GetCreatedMeshes))
  (Private|SpawnText))

(fn SetCharacterMesh
  (params (CurrentCharacter :type String))
  (bind _font (Variables|Default|GetFont))
  (bind _returnvalue (Utilities|Select :Index _font :NewEnumerator2 "/Game/ZText/Blueprints/FontTables/AudioWideTable.AudioWideTable" :NewEnumerator3 "/Game/ZText/Blueprints/FontTables/FreckleFaceTable.FreckleFaceTable" :NewEnumerator4 "/Game/ZText/Blueprints/FontTables/JollyLodgerTable.JollyLodgerTable" :NewEnumerator5 "/Game/ZText/Blueprints/FontTables/MontserratTable.MontserratTable" :NewEnumerator1 "/Game/ZText/Blueprints/FontTables/OpenSansTable.OpenSansTable" :NewEnumerator6 "/Game/ZText/Blueprints/FontTables/PressStart2PTable.PressStart2PTable" :NewEnumerator7 "/Game/ZText/Blueprints/FontTables/RobotoCondensedTable.RobotoCondensedTable" :NewEnumerator8 "/Game/ZText/Blueprints/FontTables/RussoOneTable.RussoOneTable"))
  ;[0 0 0] Match the current letter in the text to the correct character mesh for the selected font.
  (bind _outrownames (DataTable|GetDataTableRowNames _returnvalue))
  (for _array_element _outrownames
    (bind _returnvalue_2 (Utilities|GetDataTableRow _returnvalue _array_element)
      (:then
        (if (Utilities|Enum|Equal(Enum) (.String (Utilities|Struct|BreakCharacter _returnvalue_2)) CurrentCharacter)
          (return (.Mesh (Utilities|Struct|BreakCharacter _returnvalue_2)))))))
  (return (.Mesh (Utilities|Struct|BreakCharacter _returnvalue_2))))

(fn UpdateText
  (params (NewText :type Array%20of%20Strings))
  (Variables|Default|SetText NewText)
  (Private|DestroySpawnedMeshes)
  (Private|SpawnText))

(fn UpdateFont
  (params (NewFont :type DefinedFonts%20Enum :default "NewEnumerator2"))
  (Variables|Default|SetFont NewFont)
  (CallFunction|UpdateText (Variables|Default|GetText)))

(fn DestroySpawnedMeshes
  (bind _createdmeshes (Variables|Default|GetCreatedMeshes))
  ;[0 0 0] Loop over all meshes in the CreatedMeshes array. Delete them, then clear the array.
  (if (> (Utilities|Array|Length _createdmeshes) 0)
    (for _array_element _createdmeshes
      (if (not (Class|ActorComponent|IsBeingDestroyed _array_element))
        (Components|DestroyComponent _array_element)))
    (Utilities|Array|Clear _createdmeshes))
  (return))

(fn SpawnText
  (bind _returnvalue (|(({83FC7FA1-49E3-AD97-5254-68ADD4FAE50D}/2)+{3F2C9803-4523-3126-847D-E48ED570DECB})))
  (if (> (Utilities|Array|Length (Variables|Default|GetText)) 0)
    ;[0 0 0] For each line
    (for (_array_element _array_index) (Variables|Default|GetText)
      (Variables|Private|SetCurrentLine _array_index)
      ;[0 0 0] If there's anything on the line
      (if (> (Utilities|String|Len _array_element) 0)
        ;[0 0 0] For each character on the line
        (for (_array_element_2 _array_index_2) (Utilities|String|GetCharacterArrayfromString _array_element)
          (Variables|Private|SetCurrentIndex _array_index_2)
          (if (Utilities|Enum|Equal(Enum) _array_element_2 " ") ; Space character?
            ;[0 0 0] Add a space
            (Variables|Private|SetCurrentOffset (+ (Variables|Private|GetCurrentOffset) (Variables|Default|GetSpaceWidth)))
            (else
              ;[0 0 0] Spawn the 3d character staticmesh and assign material
              (bind _returnvalue_2 (AddComponent|AddStaticMeshComponent false))
              (Variables|Default|SetCurrentMesh _returnvalue_2)
              (bind _mesh (Private|SetCharacterMesh _array_element_2))
              (Components|StaticMesh|SetStaticMesh (Variables|Default|GetCurrentMesh) _mesh)
              (Rendering|Material|SetMaterial (Variables|Default|GetCurrentMesh) 0 (Variables|Default|GetTextMaterial))
              (Utilities|Array|Add (Variables|Default|GetCreatedMeshes) (Variables|Default|GetCurrentMesh))
              (Variables|Private|SetCurrentCharacterWidth (.Y (Math|Vector|BreakVector (- (.Max (Utilities|Struct|BreakBox (StaticMesh|GetBoundingBox (Variables|/Script/Engine.StaticMeshComponent|GetStaticMesh (Variables|Default|GetCurrentMesh))))) (.Min (Utilities|Struct|BreakBox (StaticMesh|GetBoundingBox (Variables|/Script/Engine.StaticMeshComponent|GetStaticMesh (Variables|Default|GetCurrentMesh)))))))))
              (if (== (Variables|Private|GetCurrentIndex) 0) ; First character?
                ;[0 0 0] First character Y offset
                (Variables|Private|SetCurrentOffset _returnvalue)
                ;;[0 0 0] Stored for alignment purposes
                (Variables|Private|SetHalfFirstCharacterWidth _returnvalue)
                (else
                  ;[0 0 0] Y offset
                  (Transformation|AddLocalOffset (Variables|Default|GetCurrentMesh) (Math|Vector|MakeVector 0.0 (|({F0FD48FE-4C5F-C333-EC27-8BBC104EE980}+({83FC7FA1-49E3-AD97-5254-68ADD4FAE50D}/2))) 0.0) false false)
                  (Variables|Private|SetCurrentOffset (|(({F0FD48FE-4C5F-C333-EC27-8BBC104EE980}+{83FC7FA1-49E3-AD97-5254-68ADD4FAE50D})+{3F2C9803-4523-3126-847D-E48ED570DECB})))))
              ;[0 0 0] Lineheight offset
              (Transformation|AddLocalOffset (Variables|Default|GetCurrentMesh) (Math|Vector|MakeVector 0.0 0.0 (|(0-({83B605CD-472B-7351-C081-9F913009E00B}*{32408ED8-41F7-AF7D-386E-E8B43CBBDF9B})))) false false)
              ;[0 0 0] Stored for alignment purposes
              (Utilities|Array|Add (Variables|Private|GetCurrentLineMeshes) (Variables|Default|GetCurrentMesh)))))
        ;[0 0 0] Line complete, perform text alignment
        (switch Utilities|FlowControl|Switch|SwitchonAlignments (Variables|Default|GetTextAlignment)
          (:NewEnumerator0
            (Variables|Private|SetAlignmentOffset (- (Variables|Private|GetHalfFirstCharacterWidth) (Variables|Default|GetKerning))))
          (:NewEnumerator1
            (Variables|Private|SetAlignmentOffset (|(0-(({F0FD48FE-4C5F-C333-EC27-8BBC104EE980}-{A9614637-420A-CC56-30F5-A9A11995D124})/2)))))
          (:NewEnumerator2
            (Variables|Private|SetAlignmentOffset (|(0-({F0FD48FE-4C5F-C333-EC27-8BBC104EE980}-{3F2C9803-4523-3126-847D-E48ED570DECB}))))))
        (for _array_element_3 (Variables|Private|GetCurrentLineMeshes)
          (Transformation|AddLocalOffset _array_element_3 (Math|Vector|MakeVector 0.0 (Variables|Private|GetAlignmentOffset) 0.0) false false))
        (Utilities|Array|Clear (Variables|Private|GetCurrentLineMeshes))))))